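; P-switch block for a platformer that the player triggers by landing on top of it, temporarily switching tagged blocks.
; A vertical hit-normal check bounces the player, plays sound, camera shake and rumble, and swaps in the smashed mesh.
; It calls PBlockOn on tagged BP_Block_base actors and starts music, then a timer calls PBlockOff on surviving blocks and stops the music.
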(event OnComponentHit(Box)
  (params (HitComponent :type Primitive%20Component%20Object%20Reference) (OtherActor :type Actor%20Object%20Reference) (OtherComp :type Primitive%20Component%20Object%20Reference) (NormalImpulse :type Vector :default "0, 0, 0") (Hit :type Hit%20Result%20Structure%20%28by%20ref%29))
  (bind _returnvalue (Game|GetPlayerCharacter 0))
  (if (and (== OtherActor _returnvalue) (Utilities|Operators|EqualEqual (.ImpactNormal (Collision|BreakHitResult Hit)) "0.000000,0.000000,-1.000000" 0.01))
    (Character|LaunchCharacter _returnvalue "0.000000,0.000000,400.000000" false false)
    (Utilities|FlowControl|Sequence
      (:then_0
        (Audio|PlaySound2D "/Game/Platformer/Audio/Mario_Thwomp.Mario_Thwomp" 1.0 1.0 0.0 0 0)
        (Audio|Components|Audio|Play (Variables|Default|GetMusic) 0.0))
      (:then_1
        (Camera|PlayWorldCameraShake "/Game/Platformer/Blueprints/BP_CameraShake.BP_CameraShake_C" (Transformation|GetActorLocation (Game|GetPlayerCharacter 0)) 1e+03 2e+03)
        (Game|Feedback|ClientPlayForceFeedback (Game|GetPlayerController 0) "/Game/Platformer/Blueprints/ForceFeedback.ForceFeedback" "None" false false false))
      (:then_2
        (Rendering|SetVisibility (Variables|Default|GetBlock_pTop_smashed) true false)
        (Components|DestroyComponent (Variables|Default|GetBox)))
      (:then_3
        (bind _outactors (Actor|GetAllActorswithTag (Variables|Default|Gettag)))
        (bind _output_get (Variables|Default|Setblocks _outactors))
        (for _array_element _output_get
          (bind _asbp_block_base (Utilities|Casting|CastToBP_Block_base _array_element))
          (Default|PBlockon _asbp_block_base)))
      (:then_4
        (Utilities|Time|SetTimerbyEvent (delegate Custom|P%20Block%20time%20over) (Variables|Default|GetPblock_timeduration))))))

(event Custom|P%20Block%20time%20over
  (for _array_element (Variables|Default|Getblocks)
    (bind _asbp_block_base (Utilities|Casting|CastToBP_Block_base _array_element))
    (Utilities|IsValid _asbp_block_base
      (:Is%20Valid
        (Default|PBlockOff _asbp_block_base))
      (:Is%20Not%20Valid
        _))
    (Audio|Components|Audio|Stop (Variables|Default|GetMusic))))

(event EventBeginPlay)

(event Collision|EventActorBeginOverlap
  (params (OtherActor :type Actor%20Object%20Reference)))

(event EventTick
  (params (DeltaSeconds :type Float%20%28single-precision%29)))

(fn ConstructionScript)