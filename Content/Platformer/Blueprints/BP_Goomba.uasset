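; BP_Goomba is a Goomba-style flipbook enemy that damages the player on overlap and dies to stomps or fireballs, awarding points.
; A detection range gates Tick movement: it either seeks the player or walks horizontally, reversing on wall hits via a debounced FlipFlop.
; Top-down hits on the Stompbox squash the sprite before destruction.
; The construction script sets walk speed and derives the flipbook play rate from it.
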(event OnComponentBeginOverlap(Collider)
  (params (OverlappedComponent :type Primitive%20Component%20Object%20Reference) (OtherActor :type Actor%20Object%20Reference) (OtherComp :type Primitive%20Component%20Object%20Reference) (OtherBodyIndex :type Integer) (bFromSweep :type Boolean) (SweepResult :type Hit%20Result%20Structure%20%28by%20ref%29))
  (bind _asbp_third_person_character (Utilities|Casting|CastToBP_ThirdPersonCharacter OtherActor))
  (Default|AdjustHitPoints _asbp_third_person_character (Variables|Default|GetHealth%20to%20substract)))

(event OnComponentHit(Stompbox)
  (params (HitComponent :type Primitive%20Component%20Object%20Reference) (OtherActor :type Actor%20Object%20Reference) (OtherComp :type Primitive%20Component%20Object%20Reference) (NormalImpulse :type Vector :default "0, 0, 0") (Hit :type Hit%20Result%20Structure%20%28by%20ref%29))
  (bind _paperflipbook (Variables|Default|GetPaperFlipbook))
  (if (and (== OtherActor (Game|GetPlayerCharacter 0)) (Utilities|Operators|EqualEqual (.ImpactNormal (Collision|BreakHitResult Hit)) "0.000000,0.000000,-1.000000" 0.1))
    (Utilities|FlowControl|Sequence
      (:then_0
        (Audio|PlaySound2D "/Game/Platformer/Audio/Mario_Squish.Mario_Squish" 1.0 1.0 0.0 0 0)
        (Collision|SetCollisionEnabled (Variables|Default|GetCollider) "NoCollision")
        (Components|DestroyComponent (Variables|Default|GetStompbox))
        (Transformation|SetWorldScale3D _paperflipbook "0.250000,0.250000,0.100000")
        (Transformation|AddWorldOffset _paperflipbook "0.000000,0.000000,-35.000000" false false)
        (Pawn|Components|CharacterMovement|DisableMovement (Variables|Character|GetCharacterMovement)))
      (:then_1
        (Game|SpawnActorfromClass "/Game/Platformer/Blueprints/BP_Points.BP_Points_C" (Transformation|GetActorTransform) "Undefined" "MultiplyWithRoot" 0 (Variables|Default|GetPoints) 0)
        (Default|AddPoints (Variables|Default|GetPlayer%20Controller) (Variables|Default|GetPoints)))
      (:then_2
        (Utilities|FlowControl|Delay 0.2)
        (Actor|DestroyActor)))))

(event OnComponentHit(Collider)
  (params (HitComponent :type Primitive%20Component%20Object%20Reference) (OtherActor :type Actor%20Object%20Reference) (OtherComp :type Primitive%20Component%20Object%20Reference) (NormalImpulse :type Vector :default "0, 0, 0") (Hit :type Hit%20Result%20Structure%20%28by%20ref%29))
  (bind _asbp_fire_ball (Utilities|Casting|CastToBP_FireBall OtherActor))
  (Actor|DestroyActor _asbp_fire_ball)
  (Utilities|FlowControl|Sequence
    (:then_0
      (Game|SpawnActorfromClass "/Game/Platformer/Blueprints/BP_Points.BP_Points_C" (Transformation|GetActorTransform) "Undefined" "MultiplyWithRoot" 0 (Variables|Default|GetPoints) 0)
      (Default|AddPoints (Variables|Default|GetPlayer%20Controller) (Variables|Default|GetPoints)))
    (:then_1
      (Utilities|FlowControl|Delay 0.2)
      (Actor|DestroyActor))))

(event OnComponentBeginOverlap(PlayerdetecRange)
  (params (OverlappedComponent :type Primitive%20Component%20Object%20Reference) (OtherActor :type Actor%20Object%20Reference) (OtherComp :type Primitive%20Component%20Object%20Reference) (OtherBodyIndex :type Integer) (bFromSweep :type Boolean) (SweepResult :type Hit%20Result%20Structure%20%28by%20ref%29))
  (if (== OtherActor (Game|GetPlayerCharacter 0))
    (Utilities|FlowControl|Gate true) ; enters at Open
  ))

(event OnComponentEndOverlap(PlayerdetecRange)
  (params (OverlappedComponent :type Primitive%20Component%20Object%20Reference) (OtherActor :type Actor%20Object%20Reference) (OtherComp :type Primitive%20Component%20Object%20Reference) (OtherBodyIndex :type Integer))
  (if (== (Game|GetPlayerCharacter 0) OtherActor)
    (Utilities|FlowControl|Gate true) ; enters at Close
  ))

(event OnComponentHit(CapsuleComponent)
  (params (HitComponent :type Primitive%20Component%20Object%20Reference) (OtherActor :type Actor%20Object%20Reference) (OtherComp :type Primitive%20Component%20Object%20Reference) (NormalImpulse :type Vector :default "0, 0, 0") (Hit :type Hit%20Result%20Structure%20%28by%20ref%29))
  (Utilities|FlowControl|DoOnce false :!label _label
    (:Completed
      (if (Utilities|Operators|EqualEqual (Math|Vector|VectorGetAbs (.ImpactNormal (Collision|BreakHitResult Hit))) "1.000000,0.000000,0.000000" 0.1)
        (Utilities|FlowControl|FlipFlop
          (:A
            (Variables|Default|SetMove%20left false))
          (:B
            (Variables|Default|SetMove%20left true)))
        (Utilities|FlowControl|Delay 0.5)
        (goto _label Reset)))))

(event EventBeginPlay
  (bind _asbp_player_controller (Utilities|Casting|CastToBP_PlayerController (Game|GetPlayerController 0)))
  (Variables|Default|SetPlayer%20Controller _asbp_player_controller))

(event Collision|EventActorBeginOverlap
  (params (OtherActor :type Actor%20Object%20Reference)))

(event EventTick
  (params (DeltaSeconds :type Float%20%28single-precision%29))
  (Utilities|FlowControl|Gate true
    (:Exit
      (if (Variables|Default|GetSeeker%20Enemy)
        (AI|Navigation|SimpleMovetoActor (Pawn|GetController) (Game|GetPlayerCharacter 0))
        (else
          (Pawn|Input|AddMovementInput (select (Variables|Default|GetMove%20left) "-1.000000,0.000000,0.000000" "1.000000,0.000000,0.000000") 1.0 false)
          (Components|Timeline|SetPlayRate (Variables|Default|GetPaperFlipbook) (Variables|Default|GetFlipbook%20play%20rate%20multiplier)))))))

(fn ConstructionScript
  (bind _output_get (Variables|/Script/Engine.CharacterMovementComponent|SetMaxWalkSpeed (Variables|Character|GetCharacterMovement) (Variables|Default|GetSpeed)))
  (Variables|Default|SetFlipbook%20play%20rate%20multiplier (Math|Float|Clamp(Float) (/ _output_get 1e+02) 0.1 3.0)))