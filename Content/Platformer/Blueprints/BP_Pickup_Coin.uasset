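; BP_Pickup_Coin is a coin pickup for a platformer that credits the player with coins when collected.
; On BeginPlay it caches the first player controller, cast to BP_PlayerController.
; When the player character overlaps its Sphere, it passes CoinstoAdd to the controller's AddCoin, plays a 2D coin sound, spawns an explosion emitter at its location and destroys itself.
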(event OnComponentBeginOverlap(Sphere)
  (params (OverlappedComponent :type Primitive%20Component%20Object%20Reference) (OtherActor :type Actor%20Object%20Reference) (OtherComp :type Primitive%20Component%20Object%20Reference) (OtherBodyIndex :type Integer) (bFromSweep :type Boolean) (SweepResult :type Hit%20Result%20Structure%20%28by%20ref%29))
  ;[1 1 1] monedas a coger
  (if (== OtherActor (Game|GetPlayerCharacter 0))
    (Default|AddCoin (Variables|Default|GetPlayer%20Controller) (Variables|Default|GetCoinsto%20Add))
    (Audio|PlaySound2D "/Game/Platformer/Audio/Mario_Coin.Mario_Coin" 1.0 1.0 0.0 0 0)
    (Effects|SpawnEmitteratLocation "/Game/StarterContent/Particles/P_Explosion.P_Explosion" (Transformation|GetActorLocation))
    (Actor|DestroyActor)))

(event EventBeginPlay
  (bind _asbp_player_controller (Utilities|Casting|CastToBP_PlayerController (Game|GetPlayerController 0)))
  (Variables|Default|SetPlayer%20Controller _asbp_player_controller))

(event Collision|EventActorBeginOverlap
  (params (OtherActor :type Actor%20Object%20Reference)))

(event EventTick
  (params (DeltaSeconds :type Float%20%28single-precision%29)))

(fn ConstructionScript)