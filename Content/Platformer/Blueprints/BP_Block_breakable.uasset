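; A breakable block for a platformer that reacts when hit, based on the player character's HitPoints.
; At two or more HitPoints, HitBlock plays the interact sound, spawns a BP_Points actor, adds points through the player controller and destroys the block.
; Otherwise it plays the Mario_BrickBreak sound and runs a timeline that moves the cube along its relative Z as a bump.
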(event EventBeginPlay
  (|CallParentFunction) ; This node is disabled and will not be called.\nDrag off pins to build functionality.
)

(event EventHitBlock
  (bind _asbp_third_person_character (Utilities|Casting|CastToBP_ThirdPersonCharacter (Game|GetPlayerCharacter 0)))
  (if (>= (Variables|/Game/ThirdPerson/Blueprints/BP_ThirdPersonCharacter.BP_ThirdPersonCharacter_C|GetHit%20Points _asbp_third_person_character) 2)
    (Utilities|FlowControl|Sequence
      (:then_0
        (Audio|PlaySound2D (Variables|Default|Getinteract%20SFX) 1.0 1.0 0.0 0 0))
      (:then_1
        (Game|SpawnActorfromClass "/Game/Platformer/Blueprints/BP_Points.BP_Points_C" (Transformation|GetActorTransform) "Undefined" "MultiplyWithRoot" 0 (Variables|Default|GetPoints) 0)
        (Default|AddPoints (Variables|Default|GetPlayer%20Controller) (Variables|Default|GetPoints)))
      (:then_2
        (Actor|DestroyActor)))
    (else
      (Audio|PlaySound2D "/Game/Platformer/Audio/Mario_BrickBreak.Mario_BrickBreak" 1.0 1.0 0.0 0 0)
      (bind _movement (Timeline|Timeline PlayFromStart)
        (:Update
          (Transformation|SetRelativeLocation (Variables|Default|GetCube) (Math|Vector|MakeVector 0.0 0.0 _movement) false false))))))

(fn ConstructionScript
  (|CallParentFunction))