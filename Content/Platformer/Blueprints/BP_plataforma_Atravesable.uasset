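; BP_plataforma_Atravesable is a one-way platform for a platformer that the player can jump up through or drop down from.
; Overlapping CollisionBottom disables the Platform's collision for player 0's character, and leaving that volume restores it.
; CollisionTop tracks whether the player stands on top, letting the IA_PlayerDowm input disable collision to drop through.
; Collision toggles on the whole Platform component, so it affects every actor, not just the player.
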(event OnComponentBeginOverlap(CollisionBottom)
  (params (OverlappedComponent :type Primitive%20Component%20Object%20Reference) (OtherActor :type Actor%20Object%20Reference) (OtherComp :type Primitive%20Component%20Object%20Reference) (OtherBodyIndex :type Integer) (bFromSweep :type Boolean) (SweepResult :type Hit%20Result%20Structure%20%28by%20ref%29))
  ;[1 1 1] Saltar a traves de plataforma
  (if (== OtherActor (Game|GetPlayerCharacter 0))
    (Collision|SetCollisionEnabled (Variables|Default|GetPlatform) "NoCollision")))

(event OnComponentEndOverlap(CollisionBottom)
  (params (OverlappedComponent :type Primitive%20Component%20Object%20Reference) (OtherActor :type Actor%20Object%20Reference) (OtherComp :type Primitive%20Component%20Object%20Reference) (OtherBodyIndex :type Integer))
  ;[1 1 1] Saltar a traves de plataforma
  (if (== (Game|GetPlayerCharacter 0) OtherActor)
    (Collision|SetCollisionEnabled (Variables|Default|GetPlatform) "QueryAndPhysics")))

(event OnComponentBeginOverlap(CollisionTop)
  (params (OverlappedComponent :type Primitive%20Component%20Object%20Reference) (OtherActor :type Actor%20Object%20Reference) (OtherComp :type Primitive%20Component%20Object%20Reference) (OtherBodyIndex :type Integer) (bFromSweep :type Boolean) (SweepResult :type Hit%20Result%20Structure%20%28by%20ref%29))
  ;[1 1 1] Set boolean for detecting if player is top of the platform
  (if (== OtherActor (Game|GetPlayerCharacter 0))
    (Variables|Default|SetIsOnTopPlatform true)))

(event OnComponentEndOverlap(CollisionTop)
  (params (OverlappedComponent :type Primitive%20Component%20Object%20Reference) (OtherActor :type Actor%20Object%20Reference) (OtherComp :type Primitive%20Component%20Object%20Reference) (OtherBodyIndex :type Integer))
  ;[1 1 1] Set boolean for detecting if player is top of the platform
  (if (== (Game|GetPlayerCharacter 0) OtherActor)
    (Variables|Default|SetIsOnTopPlatform false)))

(event Input|EnhancedActionEvents|EnhancedInputActionIA_PlayerDowm
  (params (ActionValue :type Boolean) (ElapsedSeconds :type Float%20%28double-precision%29) (TriggeredSeconds :type Float%20%28double-precision%29) (InputAction :type Input%20Action%20Object%20Reference :default "/Game/ThirdPerson/Input/Actions/IA_PlayerDowm.IA_PlayerDowm"))
  ;[1 1 1] allow player to drop dowm
  (:Started
    (if (Variables|Default|GetIsOnTopPlatform)
      (Collision|SetCollisionEnabled (Variables|Default|GetPlatform) "NoCollision"))))

(event EventBeginPlay)

(event Collision|EventActorBeginOverlap
  (params (OtherActor :type Actor%20Object%20Reference)))

(event EventTick
  (params (DeltaSeconds :type Float%20%28single-precision%29)))

(fn ConstructionScript)