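; Invisible coin block for a Mario-style platformer, derived from a parent block, that stays hidden until hit.
; BeginPlay hides the cube, ignores a custom trace channel and removes inherited child actor and coin collider.
; A box trigger disables cube collision while the player overlaps it.
; The first hit reveals the block, restores blocking, awards coins and points, and plays a timeline bump; later hits only play a sound.
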(event OnComponentBeginOverlap(Box)
  (params (OverlappedComponent :type Primitive%20Component%20Object%20Reference) (OtherActor :type Actor%20Object%20Reference) (OtherComp :type Primitive%20Component%20Object%20Reference) (OtherBodyIndex :type Integer) (bFromSweep :type Boolean) (SweepResult :type Hit%20Result%20Structure%20%28by%20ref%29))
  (if (== OtherActor (Game|GetPlayerCharacter 0))
    (Collision|SetCollisionEnabled (Variables|Default|GetCube) "NoCollision")))

(event OnComponentEndOverlap(Box)
  (params (OverlappedComponent :type Primitive%20Component%20Object%20Reference) (OtherActor :type Actor%20Object%20Reference) (OtherComp :type Primitive%20Component%20Object%20Reference) (OtherBodyIndex :type Integer))
  (if (== OtherActor (Game|GetPlayerCharacter 0))
    (Collision|SetCollisionEnabled (Variables|Default|GetCube) "QueryAndPhysics")))

(event EventBeginPlay
  (bind _cube (Variables|Default|GetCube))
  (|CallParentFunction)
  (Utilities|FlowControl|Sequence
    (:then_0
      (Rendering|SetVisibility _cube false false)
      (Collision|SetCollisionResponsetoChannel _cube "ECC_GameTraceChannel1" "ECR_Ignore"))
    (:then_1
      (Components|DestroyComponent (Variables|Default|GetChildActor)))))

(event EventHitBlock
  (bind _cube (Variables|Default|GetCube))
  (if (Variables|Default|GetFinishedInteracting)
    (Audio|PlaySound2D "/Game/Platformer/Audio/Mario_BrickBump.Mario_BrickBump" 1.0 1.0 0.0 0 0)
    (else
      (Utilities|FlowControl|Sequence
        (:then_0
          (Audio|PlaySound2D (Variables|Default|Getinteract%20SFX) 1.0 1.0 0.0 0 0)
          (Rendering|Material|SetMaterial (Variables|Default|GetCube) 0 (Variables|Default|GetMaterial)))
        (:then_1
          (Game|SpawnActorfromClass "/Game/Platformer/Blueprints/BP_Points.BP_Points_C" (Transformation|GetActorTransform) "Undefined" "MultiplyWithRoot" 0 (Variables|Default|GetPoints) 0)
          (Default|AddPoints (Variables|Default|GetPlayer%20Controller) (Variables|Default|GetPoints)))
        (:then_2
          (Game|SpawnActorfromClass "/Game/Platformer/Blueprints/BP_Block_Coin.BP_Block_Coin_C" (Transformation|GetActorTransform) "Undefined" "MultiplyWithRoot" 0 0)
          (Default|AddCoin (Variables|Default|GetPlayer%20Controller) (Variables|Default|GetCoins%20to%20add)))
        (:then_3
          (bind _movement (Timeline|BlockAnim PlayFromStart)
            (:Update
              (Transformation|SetRelativeLocation (Variables|Default|GetCube) (Math|Vector|MakeVector 0.0 0.0 _movement) false false))))
        (:then_4
          (Rendering|SetVisibility _cube true false)
          (Collision|SetCollisionResponsetoChannel _cube "ECC_GameTraceChannel1" "ECR_Block")
          (Components|DestroyComponent (Variables|Default|GetBox)))
        (:then_5
          (Variables|Default|SetFinishedInteracting true))))))

(fn ConstructionScript
  (|CallParentFunction))