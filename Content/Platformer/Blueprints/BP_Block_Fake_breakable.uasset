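; BP_Block_Fake_breakable is a Mario-style platformer block that pays out once when hit instead of breaking.
; The first HitBlock plays a sound, swaps the cube's material, spawns points and coin actors, and credits both to the player controller.
; A timeline bumps the cube along Z, and a FinishedInteracting flag limits later hits to a brick-bump sound.
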(event EventBeginPlay
  (|CallParentFunction) ; This node is disabled and will not be called.\nDrag off pins to build functionality.
)

(event EventHitBlock
  (if (Variables|Default|GetFinishedInteracting)
    (Audio|PlaySound2D "/Game/Platformer/Audio/Mario_BrickBump.Mario_BrickBump" 1.0 1.0 0.0 0 0)
    (else
      (Utilities|FlowControl|Sequence
        (:then_0
          (Audio|PlaySound2D (Variables|Default|Getinteract%20SFX) 1.0 1.0 0.0 0 0)
          (Rendering|Material|SetMaterial (Variables|Default|GetCube) 0 (Variables|Default|GetMaterial)))
        (:then_1
          (Game|SpawnActorfromClass "/Game/Platformer/Blueprints/BP_Points.BP_Points_C" (Transformation|GetActorTransform) "Undefined" "MultiplyWithRoot" 0 (Variables|Default|GetPoints) 0)
          (Default|AddPoints (Variables|Default|GetPlayer%20Controller) (Variables|Default|GetPoints)))
        (:then_2
          (Game|SpawnActorfromClass "/Game/Platformer/Blueprints/BP_Block_Coin.BP_Block_Coin_C" (Transformation|GetActorTransform) "Undefined" "MultiplyWithRoot" 0 0)
          (Default|AddCoin (Variables|Default|GetPlayer%20Controller) (Variables|Default|GetCoins%20to%20add)))
        (:then_3
          (bind _movement (Timeline|BlockAnim PlayFromStart)
            (:Update
              (Transformation|SetRelativeLocation (Variables|Default|GetCube) (Math|Vector|MakeVector 0.0 0.0 _movement) false false))))
        (:then_4
          (Variables|Default|SetFinishedInteracting true))))))

(fn ConstructionScript
  (|CallParentFunction))