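; Mushroom launcher platform that bounces the player character upward or along a configurable launch velocity.
; A straight-down hit normal on the cap triggers a once-gated launch and a timeline scale animation, whose updates re-arm the gate after a short delay.
; A bottom overlap volume disables cap collision while the player is inside, allowing passage from below.
; The construction script sizes the cap and stacks instanced trunk segments downward from TrunkEndPoint's length.
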(event OnComponentBeginOverlap(CollisionBottom)
  (params (OverlappedComponent :type Primitive%20Component%20Object%20Reference) (OtherActor :type Actor%20Object%20Reference) (OtherComp :type Primitive%20Component%20Object%20Reference) (OtherBodyIndex :type Integer) (bFromSweep :type Boolean) (SweepResult :type Hit%20Result%20Structure%20%28by%20ref%29))
  (if (== OtherActor (Game|GetPlayerCharacter 0))
    (Collision|SetCollisionEnabled (Variables|Default|GetMushTop) "NoCollision")))

(event OnComponentEndOverlap(CollisionBottom)
  (params (OverlappedComponent :type Primitive%20Component%20Object%20Reference) (OtherActor :type Actor%20Object%20Reference) (OtherComp :type Primitive%20Component%20Object%20Reference) (OtherBodyIndex :type Integer))
  (if (== (Game|GetPlayerCharacter 0) OtherActor)
    (Collision|SetCollisionEnabled (Variables|Default|GetMushTop) "QueryAndPhysics")))

(event OnComponentHit(MushTop)
  (params (HitComponent :type Primitive%20Component%20Object%20Reference) (OtherActor :type Actor%20Object%20Reference) (OtherComp :type Primitive%20Component%20Object%20Reference) (NormalImpulse :type Vector :default "0, 0, 0") (Hit :type Hit%20Result%20Structure%20%28by%20ref%29))
  (bind _returnvalue (Game|GetPlayerCharacter 0))
  (if (and (== OtherActor _returnvalue) (Class|KismetMathLibrary|EqualExactlyVectorVector (.ImpactNormal (Collision|BreakHitResult Hit)) "0.000000,0.000000,-1.000000"))
    (Utilities|FlowControl|DoOnce false
      (:Completed
        (Character|LaunchCharacter _returnvalue (Variables|Default|GetLaunchVelocity) false false)
        (bind _scalemultiplier (Timeline|mushtop%20timeline PlayFromStart)
          (:Update
            (Transformation|SetRelativeScale3D (Variables|Default|GetMushTop) (Math|Vector|MakeVector (* (Variables|Default|GetMushTop_Scale_X) _scalemultiplier) (* (Variables|Default|GetMushTop_Scale_Y) _scalemultiplier) (* (Variables|Default|GetMushTop_Scale_Z) _scalemultiplier)))
            (Utilities|FlowControl|Delay 0.2)
            (CallFunction|ResetLauncher)))))))

(event Custom|reset%20launcher
  (Utilities|FlowControl|DoOnce false) ; enters at Reset
)

(event EventBeginPlay)

(event Collision|EventActorBeginOverlap
  (params (OtherActor :type Actor%20Object%20Reference)))

(event EventTick
  (params (DeltaSeconds :type Float%20%28single-precision%29)))

(fn ConstructionScript
  (Transformation|SetWorldScale3D (Variables|Default|GetMushTop) (Math|Vector|MakeVector (Variables|Default|GetMushTop_Scale_X) (Variables|Default|GetMushTop_Scale_Y) (Variables|Default|GetMushTop_Scale_Z)))
  (for _index (range 0 (Math|Float|Truncate (/ (Math|Vector|VectorLength (Variables|Default|GetTrunkEndPoint)) 1e+02)))
    (Components|InstancedStaticMesh|AddInstance (Variables|Default|GetMushTrunk) (Math|Transform|MakeTransform (Math|Vector|MakeVector 0.0 0.0 (Math|Conversions|ToFloat(Integer) (* _index -100)))) false)))