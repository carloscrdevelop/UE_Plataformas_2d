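; BP_Block_FlowerFire is a Mario-style platformer block that releases a fire flower power-up when hit.
; The first HitBlock plays a sound, swaps the cube's material and runs timelines that bump the block and move the flower; later hits only play a bump sound.
; Player overlap with the flower calls GotFlowerPower, spawns BP_Points, adds points through the PlayerController and destroys the flower components.
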(event OnComponentBeginOverlap(Box_Flower)
  (params (OverlappedComponent :type Primitive%20Component%20Object%20Reference) (OtherActor :type Actor%20Object%20Reference) (OtherComp :type Primitive%20Component%20Object%20Reference) (OtherBodyIndex :type Integer) (bFromSweep :type Boolean) (SweepResult :type Hit%20Result%20Structure%20%28by%20ref%29))
  (bind _asbp_third_person_character (Utilities|Casting|CastToBP_ThirdPersonCharacter OtherActor))
  (Default|GotFlowerPower _asbp_third_person_character)
  (Utilities|FlowControl|Sequence
    (:then_0
      (Game|SpawnActorfromClass "/Game/Platformer/Blueprints/BP_Points.BP_Points_C" (Transformation|GetWorldTransform (Variables|Default|GetArrow)) "Undefined" "MultiplyWithRoot" 0 (Variables|Default|GetPoints) 0)
      (Default|AddPoints (Variables|Default|GetPlayer%20Controller) (Variables|Default|GetPoints)))
    (:then_1
      (Components|DestroyComponent (Variables|Default|GetBox_Flower)))))

(event EventBeginPlay
  (|CallParentFunction) ; This node is disabled and will not be called.\nDrag off pins to build functionality.
)

(event EventHitBlock
  (if (Variables|Default|GetFinishedInteracting)
    (Audio|PlaySound2D "/Game/Platformer/Audio/Mario_BrickBump.Mario_BrickBump" 1.0 1.0 0.0 0 0)
    (else
      (Utilities|FlowControl|Sequence
        (:then_0
          (Audio|PlaySound2D (Variables|Default|Getinteract%20SFX) 1.0 1.0 0.0 0 0)
          (Rendering|Material|SetMaterial (Variables|Default|GetCube) 0 (Variables|Default|GetMaterial)))
        (:then_1
          (bind _movement (Timeline|BlockAnim PlayFromStart)
            (:Update
              (Transformation|SetRelativeLocation (Variables|Default|GetCube) (Math|Vector|MakeVector 0.0 0.0 _movement) false false))))
        (:then_2
          (bind _movement_2 (Timeline|FlowerTimeline Play)
            (:Update
              (bind _box_flower (Variables|Default|GetBox_Flower)
                (:then
                  (Transformation|SetRelativeLocation _box_flower (Math|Vector|MakeVector 0.0 0.0 _movement_2) false false))
                (:else)))))
        (:then_3
          (Variables|Default|SetFinishedInteracting true))))))

(fn ConstructionScript
  (|CallParentFunction))