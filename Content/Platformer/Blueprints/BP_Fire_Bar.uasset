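; BP_Fire_Bar is a rotating bar of flame balls that damages and knocks back the player in a platformer.
; The construction script stacks instanced spheres along local Z, fits the Box trigger to their span, and sets the RotatingMovement rate.
; When BP_ThirdPersonCharacter overlaps the Box, it overrides the character's velocity and adjusts hit points.
; A DoOnce reset after a delay provides the hit cooldown.
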(event OnComponentBeginOverlap(Box)
  (params (OverlappedComponent :type Primitive%20Component%20Object%20Reference) (OtherActor :type Actor%20Object%20Reference) (OtherComp :type Primitive%20Component%20Object%20Reference) (OtherBodyIndex :type Integer) (bFromSweep :type Boolean) (SweepResult :type Hit%20Result%20Structure%20%28by%20ref%29))
  (bind _asbp_third_person_character (Utilities|Casting|CastToBP_ThirdPersonCharacter OtherActor))
  (Utilities|FlowControl|DoOnce false :!label _label
    (:Completed
      (Variables|/Script/Engine.MovementComponent|SetVelocity (Variables|/Script/Engine.Character|GetCharacterMovement _asbp_third_person_character) (Variables|Default|Getplayer%20hit%20velocity))
      (Default|AdjustHitPoints _asbp_third_person_character (Variables|Default|Gethit%20points%20adjustments))
      (Utilities|FlowControl|Delay (Variables|Default|Gethit%20colddown))
      (goto _label Reset))))

(event Collision|EventActorBeginOverlap
  (params (OtherActor :type Actor%20Object%20Reference)))

(event EventTick
  (params (DeltaSeconds :type Float%20%28single-precision%29)))

(fn ConstructionScript
  (bind _box (Variables|Default|GetBox))
  (for _index (range 0 (- (Variables|barcustomization|GetFlame%20ball%20number) 1))
    (Utilities|FlowControl|Sequence
      (:then_0
        (Components|InstancedStaticMesh|AddInstance (Variables|Default|GetSphere) (Math|Transform|MakeTransform (Math|Vector|MakeVector 0.0 0.0 (Math|Conversions|ToFloat(Integer) (* _index (Variables|barcustomization|GetFlame%20ball%20distance%20apart)))) "0, 0, 0" (Variables|barcustomization|Getflame%20ball%20size)) false))
      (:then_1
        (Transformation|SetRelativeLocation _box (Math|Vector|MakeVector 0.0 0.0 (Math|Conversions|ToFloat(Integer) (/ (* _index (Variables|barcustomization|GetFlame%20ball%20distance%20apart)) 2))) false false)
        (Components|Box|SetBoxExtent _box (Math|Vector|MakeVector 1e+01 5e+01 (Math|Conversions|ToFloat(Integer) (/ (* _index (Variables|barcustomization|GetFlame%20ball%20distance%20apart)) 2))) true))
      (:then_2
        (Variables|/Script/Engine.RotatingMovementComponent|SetRotationRate (Variables|Default|GetRotatingMovement) (Variables|barcustomization|Getrotation%20rate))))))