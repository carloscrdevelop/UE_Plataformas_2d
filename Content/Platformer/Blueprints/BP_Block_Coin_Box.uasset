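; Multi-coin block in a Mario-style platformer that pays out on repeated hits for a limited time.
; Each hit spawns coin and points actors, credits the PlayerController, plays a sound and bumps the cube with a timeline.
; The first hit starts the timer; the first hit after expiry swaps the material and gives one last payout.
; Later hits only play a brick bump sound.
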(event Custom|Timer%20expired
  (Variables|Default|SetHas%20Timer%20Expired true))

(event EventBeginPlay
  (|CallParentFunction) ; This node is disabled and will not be called.\nDrag off pins to build functionality.
)

(event EventHitBlock
  (if (Variables|Default|GetFinishedInteracting)
    (Audio|PlaySound2D "/Game/Platformer/Audio/Mario_BrickBump.Mario_BrickBump" 1.0 1.0 0.0 0 0)
    (elif (Variables|Default|GetHas%20Timer%20Expired)
      (Utilities|FlowControl|DoOnce false
        (:Completed
          (Utilities|FlowControl|Sequence
            (:then_0
              (Rendering|Material|SetMaterial (Variables|Default|GetCube) 0 (Variables|Default|GetMaterial))
              (Variables|Default|SetFinishedInteracting true))
            (:then_1
              (Utilities|FlowControl|Sequence :!label _label
                (:then_0
                  (Utilities|FlowControl|DoOnce false
                    (:Completed
                      (Utilities|Time|SetTimerbyEvent (delegate Custom|Timer%20expired) (Variables|Default|GetTimer%20Amount)))))
                (:then_1
                  (Audio|PlaySound2D (Variables|Default|Getinteract%20SFX) 1.0 1.0 0.0 0 0))
                (:then_2
                  (Game|SpawnActorfromClass "/Game/Platformer/Blueprints/BP_Points.BP_Points_C" (Transformation|GetActorTransform) "Undefined" "MultiplyWithRoot" 0 (Variables|Default|GetPoints) 0)
                  (Default|AddPoints (Variables|Default|GetPlayer%20Controller) (Variables|Default|GetPoints)))
                (:then_3
                  (Game|SpawnActorfromClass "/Game/Platformer/Blueprints/BP_Block_Coin.BP_Block_Coin_C" (Transformation|GetActorTransform) "Undefined" "MultiplyWithRoot" 0 0)
                  (Default|AddCoin (Variables|Default|GetPlayer%20Controller) (Variables|Default|GetCoins%20to%20add)))
                (:then_4
                  (bind _movement (Timeline|BlockAnim PlayFromStart)
                    (:Update
                      (Transformation|SetRelativeLocation (Variables|Default|GetCube) (Math|Vector|MakeVector 0.0 0.0 _movement) false false)))))))))
      (else
        (goto _label)))))

(fn ConstructionScript
  (|CallParentFunction))