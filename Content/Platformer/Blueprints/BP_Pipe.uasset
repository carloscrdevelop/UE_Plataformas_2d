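; Mario-style warp pipe that carries the player character to a target location when up or down is pressed, matching the pipe's direction.
; Collision overlap opens a gate for the input; entering disables input and timelines move the capsule vertically into the pipe, then at the exit, with warp sounds.
; Only the rising-exit branch re-enables input.
; The construction script stacks instanced body segments downward based on PipeEndPoint's length.
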(event OnComponentBeginOverlap(collision)
  (params (OverlappedComponent :type Primitive%20Component%20Object%20Reference) (OtherActor :type Actor%20Object%20Reference) (OtherComp :type Primitive%20Component%20Object%20Reference) (OtherBodyIndex :type Integer) (bFromSweep :type Boolean) (SweepResult :type Hit%20Result%20Structure%20%28by%20ref%29))
  (bind _warp_in_point (Variables|Default|Getwarp%20In%20Point))
  (bind _warp_to_locate (Variables|Default|GetWarp%20To%20Locate))
  (bind _warp_in_point_2 (Variables|Default|Getwarp%20In%20Point))
  (bind _warp_to_locate_2 (Variables|Default|GetWarp%20To%20Locate))
  (bind _returnvalue (Transformation|GetWorldLocation _warp_in_point))
  (bind (_x _y _z) (Math|Vector|BreakVector _warp_to_locate_2))
  (bind (_x_2 _y_2 _z_2) (Math|Vector|BreakVector _warp_to_locate))
  (bind _returnvalue_2 (Transformation|GetWorldLocation _warp_in_point_2))
  (bind (_x_3 _y_3 _z_3) (Math|Vector|BreakVector _returnvalue_2))
  (bind (_x_4 _y_4 _z_4) (Math|Vector|BreakVector _returnvalue))
  (bind _asbp_third_person_character (Utilities|Casting|CastToBP_ThirdPersonCharacter OtherActor))
  (Utilities|FlowControl|Gate true) ; enters at Open
)

(event OnComponentEndOverlap(collision)
  (params (OverlappedComponent :type Primitive%20Component%20Object%20Reference) (OtherActor :type Actor%20Object%20Reference) (OtherComp :type Primitive%20Component%20Object%20Reference) (OtherBodyIndex :type Integer))
  (bind _warp_in_point (Variables|Default|Getwarp%20In%20Point))
  (bind _warp_to_locate (Variables|Default|GetWarp%20To%20Locate))
  (bind _warp_in_point_2 (Variables|Default|Getwarp%20In%20Point))
  (bind _warp_to_locate_2 (Variables|Default|GetWarp%20To%20Locate))
  (bind _returnvalue (Transformation|GetWorldLocation _warp_in_point))
  (bind (_x _y _z) (Math|Vector|BreakVector _warp_to_locate_2))
  (bind (_x_2 _y_2 _z_2) (Math|Vector|BreakVector _warp_to_locate))
  (bind _returnvalue_2 (Transformation|GetWorldLocation _warp_in_point_2))
  (bind (_x_3 _y_3 _z_3) (Math|Vector|BreakVector _returnvalue_2))
  (bind (_x_4 _y_4 _z_4) (Math|Vector|BreakVector _returnvalue))
  (Utilities|Casting|CastToBP_ThirdPersonCharacter OtherActor)
  (Utilities|FlowControl|Gate true) ; enters at Close
)

(event Input|EnhancedActionEvents|EnhancedInputActionIA_PlayerUp
  (params (ActionValue :type Boolean) (ElapsedSeconds :type Float%20%28double-precision%29) (TriggeredSeconds :type Float%20%28double-precision%29) (InputAction :type Input%20Action%20Object%20Reference :default "/Game/ThirdPerson/Input/Actions/IA_PlayerUp.IA_PlayerUp"))
  (bind _warp_in_point (Variables|Default|Getwarp%20In%20Point))
  (bind _warp_to_locate (Variables|Default|GetWarp%20To%20Locate))
  (bind _warp_in_point_2 (Variables|Default|Getwarp%20In%20Point))
  (bind _warp_to_locate_2 (Variables|Default|GetWarp%20To%20Locate))
  (bind _returnvalue (Transformation|GetWorldLocation _warp_in_point))
  (bind (_x _y _z) (Math|Vector|BreakVector _warp_to_locate_2))
  (bind (_x_2 _y_2 _z_2) (Math|Vector|BreakVector _warp_to_locate))
  (bind _returnvalue_2 (Transformation|GetWorldLocation _warp_in_point_2))
  (bind (_x_3 _y_3 _z_3) (Math|Vector|BreakVector _returnvalue_2))
  (bind (_x_4 _y_4 _z_4) (Math|Vector|BreakVector _returnvalue))
  (:Started
    (if (and (Variables|Default|GetCan%20interact) (not (Variables|Default|GetIs%20Down%20pipe)))
      (Utilities|FlowControl|Gate true
        (:Exit
          (bind _output_get (Variables|Default|SetMy%20character (stale OnComponentBeginOverlap(collision) _asbp_third_person_character)))
          (Input|DisableInput _output_get (Game|GetPlayerController 0))
          (if (Variables|Default|GetIs%20Down%20pipe)
            (Utilities|FlowControl|Sequence
              (:then_0
                (bind _movement (Timeline|Into%20Down%20Pipe PlayFromStart)
                  (:Update
                    (Transformation|SetRelativeLocationAndRotation (Variables|/Script/Engine.Character|GetCapsuleComponent (Variables|Default|GetMy%20character)) (Math|Vector|MakeVector _x_3 _y_3 (+ _z_3 _movement)) "0, 0, 0" false false))
                  (:Finished
                    (Utilities|FlowControl|Delay 0.4 :!label _label)
                    (Audio|PlaySound2D "/Game/Platformer/Audio/Mario_Warp.Mario_Warp" 1.0 1.0 0.0 0 0)
                    (if (Variables|Default|GetExit%20Rising%20up%20out%20of%20pipe)
                      (bind _movement_2 (Timeline|Timeline PlayFromStart)
                        (:Update
                          (Transformation|SetRelativeLocationAndRotation (Variables|/Script/Engine.Character|GetCapsuleComponent (Variables|Default|GetMy%20character)) (Math|Vector|MakeVector _x_2 _y_2 (+ _z_2 _movement_2)) "0, 0, 0" false false))
                        (:Finished
                          (Input|EnableInput (Game|GetPlayerCharacter 0) (Game|GetPlayerController 0))))
                      (else
                        (bind _movement_3 (Timeline|Timeline_1 PlayFromStart)
                          (:Update
                            (Transformation|SetRelativeLocationAndRotation (Variables|/Script/Engine.Character|GetCapsuleComponent (Variables|Default|GetMy%20character)) (Math|Vector|MakeVector _x _y (+ _z _movement_3)) "0, 0, 0" false false))))))))
              (:then_1
                (Utilities|FlowControl|Delay 0.2 :!label _label_2)
                (Audio|PlaySound2D "/Game/Platformer/Audio/Mario_Warp.Mario_Warp" 1.0 1.0 0.0 0 0)))
            (else
              (Utilities|FlowControl|Sequence
                (:then_0
                  (goto _label_2))
                (:then_1
                  (bind _movement_4 (Timeline|Timeline_0 PlayFromStart)
                    (:Update
                      (Transformation|SetRelativeLocationAndRotation (Variables|/Script/Engine.Character|GetCapsuleComponent (Variables|Default|GetMy%20character)) (Math|Vector|MakeVector _x_4 _y_4 (+ _z_4 _movement_4)) "0, 0, 0" false false))
                    (:Finished
                      (goto _label))))))))))))

(event Input|EnhancedActionEvents|EnhancedInputActionIA_PlayerDowm
  (params (ActionValue :type Boolean) (ElapsedSeconds :type Float%20%28double-precision%29) (TriggeredSeconds :type Float%20%28double-precision%29) (InputAction :type Input%20Action%20Object%20Reference :default "/Game/ThirdPerson/Input/Actions/IA_PlayerDowm.IA_PlayerDowm"))
  (bind _warp_in_point (Variables|Default|Getwarp%20In%20Point))
  (bind _warp_to_locate (Variables|Default|GetWarp%20To%20Locate))
  (bind _warp_in_point_2 (Variables|Default|Getwarp%20In%20Point))
  (bind _warp_to_locate_2 (Variables|Default|GetWarp%20To%20Locate))
  (bind _returnvalue (Transformation|GetWorldLocation _warp_in_point))
  (bind (_x _y _z) (Math|Vector|BreakVector _warp_to_locate_2))
  (bind (_x_2 _y_2 _z_2) (Math|Vector|BreakVector _warp_to_locate))
  (bind _returnvalue_2 (Transformation|GetWorldLocation _warp_in_point_2))
  (bind (_x_3 _y_3 _z_3) (Math|Vector|BreakVector _returnvalue_2))
  (bind (_x_4 _y_4 _z_4) (Math|Vector|BreakVector _returnvalue))
  (:Started
    (if (and (Variables|Default|GetCan%20interact) (Variables|Default|GetIs%20Down%20pipe))
      (Utilities|FlowControl|Gate true
        (:Exit
          (bind _output_get (Variables|Default|SetMy%20character (stale OnComponentBeginOverlap(collision) _asbp_third_person_character)))
          (Input|DisableInput _output_get (Game|GetPlayerController 0))
          (if (Variables|Default|GetIs%20Down%20pipe)
            (Utilities|FlowControl|Sequence
              (:then_0
                (bind _movement (Timeline|Into%20Down%20Pipe PlayFromStart)
                  (:Update
                    (Transformation|SetRelativeLocationAndRotation (Variables|/Script/Engine.Character|GetCapsuleComponent (Variables|Default|GetMy%20character)) (Math|Vector|MakeVector _x_3 _y_3 (+ _z_3 _movement)) "0, 0, 0" false false))
                  (:Finished
                    (Utilities|FlowControl|Delay 0.4 :!label _label)
                    (Audio|PlaySound2D "/Game/Platformer/Audio/Mario_Warp.Mario_Warp" 1.0 1.0 0.0 0 0)
                    (if (Variables|Default|GetExit%20Rising%20up%20out%20of%20pipe)
                      (bind _movement_2 (Timeline|Timeline PlayFromStart)
                        (:Update
                          (Transformation|SetRelativeLocationAndRotation (Variables|/Script/Engine.Character|GetCapsuleComponent (Variables|Default|GetMy%20character)) (Math|Vector|MakeVector _x_2 _y_2 (+ _z_2 _movement_2)) "0, 0, 0" false false))
                        (:Finished
                          (Input|EnableInput (Game|GetPlayerCharacter 0) (Game|GetPlayerController 0))))
                      (else
                        (bind _movement_3 (Timeline|Timeline_1 PlayFromStart)
                          (:Update
                            (Transformation|SetRelativeLocationAndRotation (Variables|/Script/Engine.Character|GetCapsuleComponent (Variables|Default|GetMy%20character)) (Math|Vector|MakeVector _x _y (+ _z _movement_3)) "0, 0, 0" false false))))))))
              (:then_1
                (Utilities|FlowControl|Delay 0.2 :!label _label_2)
                (Audio|PlaySound2D "/Game/Platformer/Audio/Mario_Warp.Mario_Warp" 1.0 1.0 0.0 0 0)))
            (else
              (Utilities|FlowControl|Sequence
                (:then_0
                  (goto _label_2))
                (:then_1
                  (bind _movement_4 (Timeline|Timeline_0 PlayFromStart)
                    (:Update
                      (Transformation|SetRelativeLocationAndRotation (Variables|/Script/Engine.Character|GetCapsuleComponent (Variables|Default|GetMy%20character)) (Math|Vector|MakeVector _x_4 _y_4 (+ _z_4 _movement_4)) "0, 0, 0" false false))
                    (:Finished
                      (goto _label))))))))))))

(fn ConstructionScript
  (for _index (range 0 (Math|Float|Truncate (/ (Math|Vector|VectorLength (Variables|Default|GetPipe%20End%20Point)) 1e+02)))
    (Components|InstancedStaticMesh|AddInstance (Variables|Default|GetPipe%20body) (Math|Transform|MakeTransform (Math|Vector|MakeVector 0.0 0.0 (Math|Conversions|ToFloat(Integer) (* _index -100)))) false)))