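; BP_Points is a floating score popup actor for the platformer that shows a points value and then removes itself.
; On BeginPlay it gets the WBP_Points widget from its widget component, plays the points animation and sets the text to PointsToAdd.
; It waits for the animation's length, then destroys itself.
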(event EventBeginPlay
  (bind _aswbp_points (Utilities|Casting|CastToWBP_Points (UserInterface|GetWidget (Variables|Default|GetWidget))))
  (UserInterface|Animation|PlayAnimation _aswbp_points (Variables|/Game/Platformer/UI/WBP_Points.WBP_Points_C|GetPoints_animation _aswbp_points) 0.0 1 "Forward" 1.0 false)
  (Rendering|Components|TextRender|SetText (Variables|/Game/Platformer/UI/WBP_Points.WBP_Points_C|GetText_points _aswbp_points) (Utilities|Text|ToText(Integer) (Variables|Default|GetPoints%20to%20add)))
  (Utilities|FlowControl|Delay (Class|WidgetAnimation|GetEndTime (Variables|/Game/Platformer/UI/WBP_Points.WBP_Points_C|GetPoints_animation _aswbp_points)))
  (Actor|DestroyActor))

(fn ConstructionScript)