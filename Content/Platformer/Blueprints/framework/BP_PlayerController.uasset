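; BP_PlayerController is the player controller for a platformer, tracking the player's coins, lives and points.
; On BeginPlay it creates the WPB_HUD widget and adds it to the viewport.
; AddCoin adds to the coin count, and on reaching 100 it subtracts 100, grants an extra life and plays a 1-up sound.
; A separate addpoints event accumulates the score.
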(event Custom|Add%20Coin
  (params (CoinstoAdd :type Integer))
  ;[1 1 1] add coins
  (if (>= (+ CoinstoAdd (Variables|Default|GetCoins)) 100)
    (Variables|Default|SetCoins (Math|Integer|Clamp(Integer) (- (+ CoinstoAdd (Variables|Default|GetCoins)) 100) 0 100))
    (Math|Integer|IncrementInt (Variables|Default|GetLives)
      (:%20%20
        (Audio|PlaySound2D "/Game/Platformer/Audio/Mario_1up.Mario_1up" 1.0 1.0 0.0 0 0)))
    (else
      (Variables|Default|SetCoins (Math|Integer|Clamp(Integer) (+ CoinstoAdd (Variables|Default|GetCoins)) 0 100)))))

(event Custom|add%20points
  (params (Points%20to%20add :type Integer))
  (Variables|Default|SetPoints (+ Points%20to%20add (Variables|Default|GetPoints))))

(event EventBeginPlay
  (bind _returnvalue (UserInterface|CreateWidget "/Game/Platformer/UI/WPB_HUD.WPB_HUD_C"))
  (UserInterface|Viewport|AddtoViewport _returnvalue 0))

(event EventTick
  (params (DeltaSeconds :type Float%20%28single-precision%29))
  ;[1 1 1] add coins
)

(fn ConstructionScript)